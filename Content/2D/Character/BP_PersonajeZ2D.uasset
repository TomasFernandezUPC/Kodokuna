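; Player character for a 2D side-scroller with walking, running, jumping and a gravity-free dash on a cooldown, driven by Enhanced Input.
; Stamina gates and pays for run, jump and dash, and looping timers restore it while idle or walking.
; Tick refreshes the exhausted and idle flags and handles death by counting it, resetting health and teleporting to the start position.
; Stamina, health and death feedback uses on-screen PrintString messages in Spanish.
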(event `self.ReceiveBeginPlay`
  (set `self.PosInicial` (`self.K2_GetActorLocation`))
  (bind _asplayer_controller (cast `PlayerController` (`self.GetController`)))
  (`EnhancedInputSubsystemInterface.AddMappingContext` (pcsubsystem `EnhancedInputLocalPlayerSubsystem` _asplayer_controller) "/Game/2D/Character/Inputs/MapingContext/IMC_Personaje2DInputs.IMC_Personaje2DInputs" 0 (struct))
  (set `self.Cantidad de muertes` 0.0)
  (set `self.EstaminaTotal` (`self.EstaminaTotal`))
  (set `self.VidaMaxima` (`self.VidaMaxima`))
  (`KismetSystemLibrary.K2_SetTimerDelegate` (delegate `EstaminaIdle`) 3.0 true)
  (`KismetSystemLibrary.K2_SetTimerDelegate` (delegate `EstaminaWalking`) 2.0 true)
  (`KismetSystemLibrary.K2_SetTimerDelegate` (delegate `NoSufEstaminaMensaje`) 1.0 true))

(event `NoSufEstaminaMensaje`
  (if (`self.SinEstamina?`)
    (`KismetSystemLibrary.PrintString` "No tienes suficiente estamina para correr" true true (struct :`R` 1.0 :`B` 0.032711 :`A` 1.0))))

(event `self.ReceiveTick`
  (params (DeltaSeconds :type "Float (single-precision)"))
  ;[1 0 0.4332 1 50] EVENT TICK CHEQUEAR COSAS
  (`self.ChequearEstamina`)
  (`self.EstaQuieto?`)
  (`self.MUERE?`))

(event `EstaminaIdle`
  (`self.IdleRecuperandoEstamina`))

(event `EstaminaWalking`
  (`self.WalkRecupernadoEstamina`)
  (`self.CorrerMensajemenosE`))

(event `EnhancedInput|/Game/2D/Character/Inputs/InputAction/IA_VerEstamina`
  (params (ActionValue :type Boolean) (ElapsedSeconds :type "Float (double-precision)") (TriggeredSeconds :type "Float (double-precision)") (InputAction :type "InputAction Object Reference" :default "/Game/2D/Character/Inputs/InputAction/IA_VerEstamina.IA_VerEstamina"))
  ;[1 0.5161 0 1 51] Ver Estamina actual del PJ
  (:`Started`
    (`KismetSystemLibrary.PrintString` (`KismetStringLibrary.Concat_StrStr` "Tu Estamina actual es de: " (`KismetStringLibrary.Conv_DoubleToString` (`self.EstaminaTotal`))) true true (struct :`R` 1.0 :`G` 0.578253 :`A` 1.0))))

(event `EnhancedInput|/Game/2D/Character/Inputs/InputAction/IA_VerVida`
  (params (ActionValue :type Boolean) (ElapsedSeconds :type "Float (double-precision)") (TriggeredSeconds :type "Float (double-precision)") (InputAction :type "InputAction Object Reference" :default "/Game/2D/Character/Inputs/InputAction/IA_VerVida.IA_VerVida"))
  ;[0.2218 1 0 1 50] Ver Vida actual del PJ
  (:`Started`
    (`KismetSystemLibrary.PrintString` (`KismetStringLibrary.Concat_StrStr` "Tu Vida actual es de: " (`KismetStringLibrary.Conv_DoubleToString` (`self.VidaMaxima`))) true true (struct :`R` 0.104679 :`G` 0.572917 :`A` 1.0))))

(event `EnhancedInput|/Game/2D/Character/Inputs/InputAction/IA_Walk`
  (params (ActionValue :type "Float (double-precision)") (ElapsedSeconds :type "Float (double-precision)") (TriggeredSeconds :type "Float (double-precision)") (InputAction :type "InputAction Object Reference" :default "/Game/2D/Character/Inputs/InputAction/IA_Walk.IA_Walk"))
  (bind _returnvalue (`self.GetController`))
  (bind _returnvalue_x (`KismetMathLibrary.BreakVector` (`CharacterMovementComponent.GetCurrentAcceleration` (`self.CharacterMovement`))))
  ;[0 0.1656 0.1373 1 50] Caminar
  (:`Triggered`
    (`self.AddMovementInput` (1.0 0.0 0.0) ActionValue)
    (set `self.IsWalking?` true)
    (`/Engine/EditorBlueprintResources/StandardMacros.CompareFloat` _returnvalue_x
      (:`>`
        (`Controller.SetControlRotation` _returnvalue (`KismetMathLibrary.MakeRotator` 0.0)))
      (:`<`
        (`Controller.SetControlRotation` _returnvalue (`KismetMathLibrary.MakeRotator` 0.0 0.0 180.0)))))
  (:`Completed`
    (set `self.IsWalking?` false)))

(event `EnhancedInput|/Game/2D/Juego/ElementosNivel/InputEscape/IA_Escape`
  (params (ActionValue :type Boolean) (ElapsedSeconds :type "Float (double-precision)") (TriggeredSeconds :type "Float (double-precision)") (InputAction :type "InputAction Object Reference" :default "/Game/2D/Juego/ElementosNivel/InputEscape/IA_Escape.IA_Escape"))
  ;[0 0.06499 1 1 50] SALIR DEL JUEGO
  (:`Triggered`
    (`KismetSystemLibrary.QuitGame` null "Quit")))

(event `EnhancedInput|/Game/2D/Character/Inputs/InputAction/IA_Run`
  (params (ActionValue :type Boolean) (ElapsedSeconds :type "Float (double-precision)") (TriggeredSeconds :type "Float (double-precision)") (InputAction :type "InputAction Object Reference" :default "/Game/2D/Character/Inputs/InputAction/IA_Run.IA_Run"))
  (bind _charactermovement (`self.CharacterMovement`))
  ;[1 0.4616 0 1 50] Correr
  (:`Triggered`
    (if (`self.SinEstamina?`)
      (set `self.IsRunning?` false)
      (set `CharacterMovementComponent.MaxWalkSpeed` 600.0 _charactermovement)
      (else
        (set `self.IsRunning?` ActionValue)
        (set `CharacterMovementComponent.MaxWalkSpeed` 1200.0 _charactermovement)
        (set `self.EstaminaTotal` (- (`self.EstaminaTotal`) 0.1)))))
  (:`Completed`
    (set `self.IsRunning?` ActionValue)
    (set `CharacterMovementComponent.MaxWalkSpeed` 600.0 _charactermovement)))

(event `EndDash`
  ;[1 0 0.05704 1 50] Dash
  (set `CharacterMovementComponent.GravityScale` 3.0 (`self.CharacterMovement`))
  (`KismetSystemLibrary.K2_ClearTimer` null "EndDash"))

(event `EnhancedInput|/Game/2D/Character/Inputs/InputAction/IA_Dash`
  (params (ActionValue :type Boolean) (ElapsedSeconds :type "Float (double-precision)") (TriggeredSeconds :type "Float (double-precision)") (InputAction :type "InputAction Object Reference" :default "/Game/2D/Character/Inputs/InputAction/IA_Dash.IA_Dash"))
  ;[1 0 0.05704 1 50] Dash
  (:`Started`
    (if (>= (`self.EstaminaTotal`) 20.0)
      (if (`self.PuedoDashear`)
        (set `self.TengoEDash` true)
        (set `self.EstaminaTotal` (- (`self.EstaminaTotal`) 20.0))
        (`KismetSystemLibrary.PrintString` "-20 de estamina al haber utilizado el dash" true true (struct :`R` 1.0 :`G` 0.010357 :`A` 1.0))
        (set `self.PuedoDashear` false)
        (set `CharacterMovementComponent.GravityScale` 0.0 (`self.CharacterMovement`))
        (`self.LaunchCharacter` (* (`self.GetActorForwardVector`) (`self.VelocidadDash`)) true true)
        (`KismetSystemLibrary.K2_SetTimerDelegate` (delegate `EndDash`) 0.2)
        (`KismetSystemLibrary.Delay` 7.0)
        (set `self.PuedoDashear` true)
        (else
          (`KismetSystemLibrary.PrintString` "Debes esperar 7 segundos luego de haber utilizado el dash" true true (struct :`R` 1.0 :`G` 0.104277 :`A` 1.0))))
      (else
        (`KismetSystemLibrary.PrintString` "No tienes suficiente estamina para dashear" true true (struct :`R` 1.0 :`B` 0.032711 :`A` 1.0))
        (set `self.TengoEDash` false))))
  (:`Completed`
    (set `self.TengoEDash` false)))

(event `EnhancedInput|/Game/2D/Character/Inputs/InputAction/IA_Jump`
  (params (ActionValue :type Boolean) (ElapsedSeconds :type "Float (double-precision)") (TriggeredSeconds :type "Float (double-precision)") (InputAction :type "InputAction Object Reference" :default "/Game/2D/Character/Inputs/InputAction/IA_Jump.IA_Jump"))
  (:`Started`
    ;[0 1 0.0242 1 50] Salto Común
    (if (`self.SinEstamina?`)
      (`KismetSystemLibrary.PrintString` "No tienes suficiente estamina para saltar" true true (struct :`R` 1.0 :`B` 0.032711 :`A` 1.0))
      (set `self.IsJumping` false)
      (elif (not (`self.IsRunning?`))
        (set `CharacterMovementComponent.JumpZVelocity` 1400.0 (`self.CharacterMovement`))
        (`self.Jump`)
        (set `self.IsJumping` true)
        (set `self.EstaminaTotal` (- (`self.EstaminaTotal`) 3.0))
        (`KismetSystemLibrary.PrintString` "-3 de estamina por saltar" true true (struct :`R` 1.0 :`B` 0.063567 :`A` 1.0))
        (else
          ;[0 1 0.2459 1 50] Salto corriendo
          (set `self.IsJumping` true)
          (set `CharacterMovementComponent.JumpZVelocity` 1900.0 (`self.CharacterMovement`))
          (`self.Jump`)
          (set `self.EstaminaTotal` (- (`self.EstaminaTotal`) 3.0))
          (`KismetSystemLibrary.PrintString` "-7 de estamina por saltar" true true (struct :`R` 1.0 :`B` 0.063567 :`A` 1.0))))))
  (:`Completed`
    (set `self.IsJumping` false)))

(fn `ChequearEstamina`
  (if (>= (`self.EstaminaTotal`) 0.0)
    (set `self.SinEstamina?` false)
    (else
      (set `self.SinEstamina?` true))))

(fn `CorrerMensajemenosE`
  (if (`self.IsRunning?`)
    (`KismetSystemLibrary.PrintString` "Recuerda que Pierdes estamina por correr" true true (struct :`R` 0.85625 :`G` 0.038181 :`A` 1.0))))

(fn `EstaQuieto?`
  (if (and (not (`self.IsWalking?`)) (not (`self.IsRunning?`)) (not (`self.IsJumping`)) (not (`self.TengoEDash`)))
    (set `self.EstaminaQuieto` true)
    (else
      (set `self.EstaminaQuieto` false))))

(fn `IdleRecuperandoEstamina`
  (bind _estaminatotal (`self.EstaminaTotal`))
  (if (`self.EstaminaQuieto`)
    (`KismetSystemLibrary.PrintString` "¡Estas Descansando!" true true (struct :`R` 1.0 :`G` 0.51509 :`A` 1.0))
    (set `self.EstaminaTotal` (+ _estaminatotal 15.0))
    (`KismetSystemLibrary.PrintString` (`KismetStringLibrary.Concat_StrStr` "Tu Estamina actual es de: " (`KismetStringLibrary.Conv_DoubleToString` _estaminatotal)) true true (struct :`R` 1.0 :`G` 0.65108 :`A` 1.0))))

(fn `MUERE?`
  (if (<= (`self.VidaMaxima`) 0.0)
    (`KismetSystemLibrary.PrintString` "TE MORISTE!!!!" true true (struct :`R` 0.951201 :`B` 1.0 :`A` 1.0) 5.0)
    (bind _output_get (set `self.Cantidad de muertes` (+ (`self.Cantidad de muertes`) 1.0)))
    (`KismetSystemLibrary.PrintString` (`KismetStringLibrary.Concat_StrStr` "HAS MUERTO UN TOTAL DE:  " (`KismetStringLibrary.Conv_DoubleToString` _output_get)) true true (struct :`R` 0.818894 :`B` 1.0 :`A` 1.0) 5.0)
    (set `self.VidaMaxima` 40.0)
    (`self.K2_SetActorLocation` (`self.PosInicial`))))

(fn `UserConstructionScript`)

(fn `WalkRecupernadoEstamina`
  (if (`self.IsWalking?`)
    (set `self.EstaminaTotal` (+ (`self.EstaminaTotal`) 5.0))))