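; BP_PruebaPersonaje is a test player character that moves along its forward axis and turns by yaw, using Enhanced Input.
; On BeginPlay, it registers the IMC_PruebaPersonajeInputs mapping context with the owning player controller's local input subsystem.
; IA_PruebaMovimiento scales movement input along the actor's forward vector, and IA_PruebaMirar feeds controller yaw, with no pitch or strafing.
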(event `self.ReceiveBeginPlay`
  (`self.AgregarMappingContext`))

(event `EnhancedInput|/Game/Pruebas/Character/Inputs/InputAction/IA_PruebaMirar`
  (params (ActionValue :type "Float (double-precision)") (ElapsedSeconds :type "Float (double-precision)") (TriggeredSeconds :type "Float (double-precision)") (InputAction :type "InputAction Object Reference" :default "/Game/Pruebas/Character/Inputs/InputAction/IA_PruebaMirar.IA_PruebaMirar"))
  (:`Triggered`
    (`self.AddControllerYawInput` ActionValue)))

(event `EnhancedInput|/Game/Pruebas/Character/Inputs/InputAction/IA_PruebaMovimiento`
  (params (ActionValue :type "Float (double-precision)") (ElapsedSeconds :type "Float (double-precision)") (TriggeredSeconds :type "Float (double-precision)") (InputAction :type "InputAction Object Reference" :default "/Game/Pruebas/Character/Inputs/InputAction/IA_PruebaMovimiento.IA_PruebaMovimiento"))
  (:`Triggered`
    (`self.AddMovementInput` (`self.GetActorForwardVector`) ActionValue)))

(fn `AgregarMappingContext`
  (bind _asplayer_controller (cast `PlayerController` (`self.GetController`)))
  (`EnhancedInputSubsystemInterface.AddMappingContext` (pcsubsystem `EnhancedInputLocalPlayerSubsystem` _asplayer_controller) "/Game/Pruebas/Character/Inputs/MapingContext/IMC_PruebaPersonajeInputs.IMC_PruebaPersonajeInputs" 0 (struct)))

(fn `UserConstructionScript`)